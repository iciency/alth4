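; BP_AltH4GameInstance is a game instance Blueprint that holds and persists the player's save data as a BP_PlayerSaveData object in UserData.
; LoadUserData reads the fixed "Test" slot, or creates a fresh save object in memory when none exists.
; SaveUserData writes UserData back to that slot.
; ResetPlayerData prints a debug message, deletes the slot and replaces UserData with a new object without saving it.
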(event `LoadUserData`
  (bind _returnvalue (`GameplayStatics.DoesSaveGameExist` "Test"))
  (if _returnvalue
    (bind _returnvalue_2 (`GameplayStatics.LoadGameFromSlot` "Test"))
    (bind _asbp_player_save_data (cast `/Game/Blueprint/BP_PlayerSaveData` _returnvalue_2))
    (set `self.UserData` _asbp_player_save_data)
    (else
      (bind _returnvalue_3 (`GameplayStatics.CreateSaveGameObject` "/Game/Blueprint/BP_PlayerSaveData.BP_PlayerSaveData_C"))
      (set `self.UserData` _returnvalue_3))))

(event `SaveUserData`
  (`GameplayStatics.SaveGameToSlot` (`self.UserData`) "Test"))

(event `ResetPlayerData`
  (`KismetSystemLibrary.PrintString` "Reset")
  (`GameplayStatics.DeleteGameInSlot` "Test")
  (bind _returnvalue (`GameplayStatics.CreateSaveGameObject` "/Game/Blueprint/BP_PlayerSaveData.BP_PlayerSaveData_C"))
  (set `self.UserData` _returnvalue))