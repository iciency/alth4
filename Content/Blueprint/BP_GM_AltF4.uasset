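; Game mode for AltF4 that handles checkpoint saving and player death and respawn.
; SavePlayer replaces the spawned BP_RespawnPoint and persists its location through the game instance's UserData.
; BeginPlay recreates a saved point and moves all third-person characters to it.
; Death increments a counter, shows the death UI and restarts the player after a delay, with overridden FindPlayerStart preferring the latest save point over the first PlayerStart.
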(event `self.ReceiveBeginPlay`
  (bind _asbp_alt_h4game_instance (cast `/Game/Blueprint/BP_AltH4GameInstance` (`GameplayStatics.GetGameInstance`)))
  (bind _userdata (`/Game/Blueprint/BP_AltH4GameInstance.UserData` _asbp_alt_h4game_instance))
  (`/Engine/EditorBlueprintResources/StandardMacros.IsValid` _userdata
    (:`Is Valid`
      (if (`/Game/Blueprint/BP_PlayerSaveData.HasSavePoint` _userdata)
        (bind _playerlocation (`/Game/Blueprint/BP_PlayerSaveData.PlayerLocation` _userdata))
        (set `self.LatestPlayerSaveLocation` _playerlocation)
        (bind _returnvalue (`|SpawnActorFromClass` "/Game/Blueprint/BP_RespawnPoint.BP_RespawnPoint_C" (`KismetMathLibrary.MakeTransform` _playerlocation) "AdjustIfPossibleButAlwaysSpawn" "OverrideRootScale" self null))
        (bind _output_get (set `self.LatestSavePoint` _returnvalue))
        (bind _outactors (`GameplayStatics.GetAllActorsOfClass` "/Game/ThirdPerson/Blueprints/BP_ThirdPersonCharacter.BP_ThirdPersonCharacter_C"))
        (for _array_element _outactors
          (`self.K2_SetActorLocation` _array_element (`self.K2_GetActorLocation` _output_get) false false))))))

(event `On Player Dead`
  (params (Controller :type "Controller Object Reference"))
  (`/Engine/EditorBlueprintResources/StandardMacros.IncrementInt` (`self.PlayerDeathCount`)
    (:`  `
      (`KismetSystemLibrary.K2_SetTimerDelegate` (delegate `On Restart Player`) 2.0)
      (bind _output_get (set `self.RestartController` Controller))
      (bind _asbp_pc (cast `/Game/Blueprint/BP_PC` _output_get))
      (`/Game/Blueprint/BP_PC.ShowDieUI` _asbp_pc true))))

(event `On Restart Player`
  (bind _restartcontroller (`self.RestartController`))
  (`KismetSystemLibrary.PrintString` "On Player Dead")
  (`self.RestartPlayer` _restartcontroller)
  (bind _asbp_pc (cast `/Game/Blueprint/BP_PC` _restartcontroller))
  (`/Game/Blueprint/BP_PC.ShowDieUI` _asbp_pc false))

(event `Save Player`
  (params (ActorLocation :type "Vector Structure"))
  (bind _latestsavepoint (`self.LatestSavePoint`))
  (`KismetSystemLibrary.PrintString` "Save Player")
  (bind _output_get (set `self.LatestPlayerSaveLocation` ActorLocation))
  (`/Engine/EditorBlueprintResources/StandardMacros.IsValid` _latestsavepoint
    (:`Is Valid`
      (`self.K2_DestroyActor` _latestsavepoint))
    (:`Is Not Valid`
      _))
  (bind _returnvalue (`|SpawnActorFromClass` "/Game/Blueprint/BP_RespawnPoint.BP_RespawnPoint_C" (`KismetMathLibrary.MakeTransform` _output_get) "AdjustIfPossibleButAlwaysSpawn" "OverrideRootScale" self null))
  (set `self.LatestSavePoint` _returnvalue)
  (bind _asbp_alt_h4game_instance (cast `/Game/Blueprint/BP_AltH4GameInstance` (`GameplayStatics.GetGameInstance`)))
  (bind _userdata (`/Game/Blueprint/BP_AltH4GameInstance.UserData` _asbp_alt_h4game_instance))
  (`/Engine/EditorBlueprintResources/StandardMacros.IsValid` _userdata
    (:`Is Valid`
      (set `/Game/Blueprint/BP_PlayerSaveData.HasSavePoint` true _userdata)
      (set `/Game/Blueprint/BP_PlayerSaveData.PlayerLocation` (`self.LatestPlayerSaveLocation`) _userdata)
      (`/Game/Blueprint/BP_AltH4GameInstance.SaveUserData` _asbp_alt_h4game_instance))))

(fn `FindPlayerStart`
  (params (Player :type "Controller Object Reference") (IncomingName :type String))
  (returns (ReturnValue :type "Actor Object Reference"))
  (`/Engine/EditorBlueprintResources/StandardMacros.IsValid` (`self.LatestSavePoint`)
    (:`Is Valid`
      (return (`self.LatestSavePoint`)))
    (:`Is Not Valid`
      (bind _outactors (`GameplayStatics.GetAllActorsOfClass` "/Script/Engine.PlayerStart"))
      (return (`|GetArrayItem` _outactors)))))

(fn `UserConstructionScript`)