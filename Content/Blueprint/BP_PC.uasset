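; BP_PC is a player controller that shows the death and success screens for its player.
; ShowDieUI creates and displays the UI_Die widget, or removes the stored instance and clears its reference when hidden.
; ShowSuccess displays UI_Success, shows the mouse cursor, blocks move and look input, and plays a success sound.
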(event `ShowDieUI`
  (params (Show :type Boolean))
  (bind _uidie (`self.UIDie`))
  (if Show
    (bind _returnvalue (`|CreateWidget` "/Game/UI/UI_Die.UI_Die_C" self))
    (bind _output_get (set `self.UIDie` _returnvalue))
    (`UserWidget.AddToViewport` _output_get 0)
    (else
      (`/Engine/EditorBlueprintResources/StandardMacros.IsValid` _uidie
        (:`Is Valid`
          (`Widget.RemoveFromParent` _uidie)
          (set `self.UIDie` null))))))

(event `Show Success`
  (bind _returnvalue (`|CreateWidget` "/Game/UI/UI_Success.UI_Success_C" self))
  (`UserWidget.AddToViewport` _returnvalue 0)
  (set `self.bShowMouseCursor` true)
  (`self.SetIgnoreMoveInput` true)
  (`self.SetIgnoreLookInput` true)
  (`GameplayStatics.PlaySound2D` "/Game/Sound/Success_1.Success_1" 1.0 1.0 0.0 null null))

(fn `UserConstructionScript`)